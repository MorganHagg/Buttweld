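; Marve_BP holds player stats (health, threat, ammo, enemies, currency) with debug keys that step them, apparently for testing PlayerHud_BP.
; Each key calls a small function applying an unclamped fixed increment or decrement.
; BeginPlay initializes health, repeatedly creates and removes a HUD widget, then displays a separate second instance.
; R and H add and remove only the first variable's widget, whose owning-player cast never runs.
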(event Collision|EventActorBeginOverlap
  (params (OtherActor :type Actor%20Object%20Reference)))

(event EventBeginPlay
  (Utilities|FlowControl|Sequence
    (:then_0
      (Variables|Default|SetHealth (Variables|Default|GetMaxHealth))
      (bind _returnvalue (UserInterface|CreateWidget "/Game/PlayerHud_BP.PlayerHud_BP_C" (stale _asplayer_controller) :!label _label))
      (Widget|RemovefromParent _returnvalue))
    (:then_1
      (Variables|Default|SetThreat (Variables|Default|GetThreat))
      (goto _label))
    (:then_2
      (Variables|Default|SetAmmo (Variables|Default|GetAmmo))
      (goto _label))
    (:then_3
      (Variables|Default|SetEnemies (Variables|Default|GetEnemies))
      (goto _label))
    (:then_4
      (Variables|Default|SetCurrency (Variables|Default|GetCurrency))
      (goto _label))
    (:then_5
      (bind _returnvalue_2 (UserInterface|CreateWidget "/Game/PlayerHud_BP.PlayerHud_BP_C"))
      (UserInterface|Viewport|AddtoViewport _returnvalue_2 0)
      (Variables|/Script/Engine.PlayerController|SetbShowMouseCursor (Game|GetPlayerController 0) false))))

(event EventTick
  (params (DeltaSeconds :type Float%20%28single-precision%29)))

(event Input|KeyboardEvents|G
  (params (Key :type Key%20Structure :default "AnyKey"))
  (:Pressed
    (CallFunction|TakeDamage)))

(event Input|KeyboardEvents|V
  (params (Key :type Key%20Structure :default "AnyKey"))
  (:Pressed
    (CallFunction|DecayThreatMeter)))

(event Input|KeyboardEvents|C
  (params (Key :type Key%20Structure :default "AnyKey"))
  (:Pressed
    (CallFunction|ThreatMeter)))

(event Input|KeyboardEvents|1
  (params (Key :type Key%20Structure :default "AnyKey"))
  (:Pressed
    (CallFunction|EnemiesIncrease)))

(event Input|KeyboardEvents|2
  (params (Key :type Key%20Structure :default "AnyKey"))
  (:Pressed
    (CallFunction|EnemiesDecrease)))

(event Input|KeyboardEvents|3
  (params (Key :type Key%20Structure :default "AnyKey"))
  (:Pressed
    (CallFunction|CurrencyIncrease)))

(event Input|KeyboardEvents|4
  (params (Key :type Key%20Structure :default "AnyKey"))
  (:Pressed
    (CallFunction|CurrencyDecrease)))

(event Input|KeyboardEvents|5
  (params (Key :type Key%20Structure :default "AnyKey"))
  (:Pressed
    (CallFunction|AmmoIncrease)))

(event Input|KeyboardEvents|6
  (params (Key :type Key%20Structure :default "AnyKey"))
  (:Pressed
    (CallFunction|AmmoDecrease)))

(event Input|KeyboardEvents|H
  (params (Key :type Key%20Structure :default "AnyKey"))
  (:Pressed
    (Widget|RemovefromParent (stale EventBeginPlay _returnvalue))))

(event Input|KeyboardEvents|R
  (params (Key :type Key%20Structure :default "AnyKey"))
  (:Pressed
    (UserInterface|Viewport|AddtoViewport (stale EventBeginPlay _returnvalue) 0)))

(event Input|KeyboardEvents|F
  (params (Key :type Key%20Structure :default "AnyKey"))
  (:Pressed
    (CallFunction|Heal)))

(fn ConstructionScript)

(fn TakeDamage
  (Variables|Default|SetHealth (- (Variables|Default|GetHealth) 5.0)))

(fn ThreatMeter
  (Variables|Default|SetThreat (+ (Variables|Default|GetThreat) 1e+01)))

(fn DecayThreatMeter
  (Variables|Default|SetThreat (- (Variables|Default|GetThreat) 1e+01)))

(fn AmmoIncrease
  (Variables|Default|SetAmmo (+ (Variables|Default|GetAmmo) 1)))

(fn AmmoDecrease
  (Variables|Default|SetAmmo (- (Variables|Default|GetAmmo) 1)))

(fn EnemiesIncrease
  (Variables|Default|SetEnemies (+ (Variables|Default|GetEnemies) 1)))

(fn EnemiesDecrease
  (Variables|Default|SetEnemies (- (Variables|Default|GetEnemies) 1)))

(fn CurrencyIncrease
  (Variables|Default|SetCurrency (+ (Variables|Default|GetCurrency) 1)))

(fn CurrencyDecrease
  (Variables|Default|SetCurrency (- (Variables|Default|GetCurrency) 1)))

(fn Heal
  (Variables|Default|SetHealth (+ (Variables|Default|GetHealth) 5.0)))