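; Marve_BP is a player-side actor that manages HUD, pause menu and end-of-game screens, plus throw and ammo state.
; BeginPlay creates the player HUD with a reference to the first Liv_BP found.
; P toggles pause and alternates via FlipFlop between the menu and a rebuilt HUD, which omits that reference.
; Tick re-adds win or loss widgets while flagged, pauses on loss, and clears IsThrowing after a delay.
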(event EventBeginPlay
  ;[1 1 1] Creates player HUD
  (bind _item (CallFunction|GetLivRef))
  (bind _returnvalue (UserInterface|CreateWidget "/Game/Blueprints/PlayerHud_BP.PlayerHud_BP_C" (stale _asplayer_controller) _item))
  (bind _output_get (Variables|Default|SetHud%20Reference _returnvalue))
  (UserInterface|Viewport|AddtoViewport _output_get 0))

(event Collision|EventActorBeginOverlap
  (params (OtherActor :type Actor%20Object%20Reference)))

(event EventTick
  (params (DeltaSeconds :type Float%20%28single-precision%29))
  (Utilities|FlowControl|Sequence
    (:then_0
      ;[1 1 1] Add guid text on win
      (if (Variables|Default|GetGameWon)
        (bind _returnvalue (UserInterface|CreateWidget "/Game/Blueprints/Progress_BP.Progress_BP_C"))
        (UserInterface|Viewport|AddtoViewport _returnvalue 0)))
    (:then_1
      ;[1 1 1] Pause game on loss
      (if (Variables|Default|GetGameLost)
        (bind _returnvalue_2 (UserInterface|CreateWidget "/Game/Blueprints/LoseHud_BP.LoseHud_BP_C"))
        (UserInterface|Viewport|AddtoViewport _returnvalue_2 0)
        (Game|SetGamePaused true)))
    (:then_2
      (if (Variables|Default|GetisThrowing)
        (Utilities|FlowControl|Delay 0.4)
        (Variables|Default|SetisThrowing false)))))

(event Input|KeyboardEvents|P
  (params (Key :type Key%20Structure :default "AnyKey"))
  (:Pressed
    (Utilities|FlowControl|Sequence
      (:then_0
        (bind _returnvalue (UserInterface|CreateWidget "/Game/Blueprints/MenuHud_BP.MenuHud_BP_C"))
        (Utilities|FlowControl|FlipFlop
          (:A
            ;[1 1 1] Adds menu-HUD
            (Utilities|FlowControl|Sequence
              (:then_0
                (Variables|/Script/Engine.PlayerController|SetbShowMouseCursor (Game|GetPlayerController 0) true))
              (:then_1
                (UserInterface|Viewport|AddtoViewport _returnvalue 0))))
          (:B
            ;[1 1 1] Removes all widgets, then adds player-HUD
            (Utilities|FlowControl|Sequence
              (:then_0
                (Viewport|RemoveAllWidgets))
              (:then_1
                (Variables|/Script/Engine.PlayerController|SetbShowMouseCursor (Game|GetPlayerController 0) false))
              (:then_2
                (bind _returnvalue_2 (UserInterface|CreateWidget "/Game/Blueprints/PlayerHud_BP.PlayerHud_BP_C" (Game|GetPlayerController 0)))
                (UserInterface|Viewport|AddtoViewport _returnvalue_2 0))))))
      (:then_1
        ;[1 1 1] Pause /Unpause game
        (if (Variables|Default|GetPauseGame)
          (bind _output_get (Variables|Default|SetPauseGame false))
          (Game|SetGamePaused _output_get)
          (else
            (bind _output_get_2 (Variables|Default|SetPauseGame true))
            (Game|SetGamePaused _output_get_2)))))))

(fn ConstructionScript)

(fn GetLivRef
  (bind _outactors (Actor|GetAllActorsOfClass "/Game/Blueprints/Liv_BP.Liv_BP_C"))
  (return (Utilities|Array|Get(acopy) _outactors)))

(fn AddAmmoMarve
  ;[1 1 1] Sets AmmoCount to 10
  (Variables|Default|SetAmmoCount (+ (Variables|Default|GetAmmoCount) (Variables|Default|GetAmmoIncline))))